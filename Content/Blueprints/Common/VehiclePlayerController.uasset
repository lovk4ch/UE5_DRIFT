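; Player controller for driving the simple car pawn, which sets up input and shows a speedometer HUD.
; On BeginPlay it adds the default Enhanced Input mapping context, creates the VehicleUI widget in km/h mode and caches the possessed BP_SimpleCar_Pawn.
; Each tick, while that car is valid, it passes the magnitude of the car's velocity to the HUD's speed display.
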(event `self.ReceiveBeginPlay`
  (`EnhancedInputSubsystemInterface.AddMappingContext` (subsystem `EnhancedInputLocalPlayerSubsystem`) "/Game/Input/IMC_Default.IMC_Default" 0 (struct)) ; Adding the Input Mapping Context needed to trigger the proper Input Actions.
  (bind _returnvalue (`|CreateWidget` "/Game/Blueprints/Common/VehicleUI.VehicleUI_C" self))
  (bind _output_get (set `self.VehicleHud` _returnvalue))
  (`UserWidget.AddToViewport` _output_get 0)
  (bind _asbp_simple_car_pawn (cast `/Game/Blueprints/SimpleCar/BP_SimpleCar_Pawn` (`self.K2_GetPawn`)))
  (set `self.Car` _asbp_simple_car_pawn))

(event `self.ReceiveTick`
  (params (DeltaSeconds :type "Float (single-precision)"))
  (bind _car (`self.Car`)
    (:`then`
      (`/Game/Blueprints/Common/VehicleUI.UpdateSpeed` (`self.VehicleHud`) (`KismetMathLibrary.VSize` (`self.GetVelocity` _car))))
    (:`else`)))

(fn `UserConstructionScript`)